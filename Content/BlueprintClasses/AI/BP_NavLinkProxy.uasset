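; Smart nav link proxy that makes the chaser statue enemy jump to the link destination when it reaches the link.
; On SmartLinkReached it casts the agent to that character, computes a jump velocity and launches it with both XY and Z overrides.
; The JumpVelocity function solves projectile motion from start, end and a set jump duration, using a hardcoded gravity value rather than the world setting.
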(event `self.ReceiveSmartLinkReached`
  (params (Agent :type "Actor Object Reference") (Destination :type "Vector Structure (by ref)"))
  (bind _asbp_ai_enemy_chaser_statue_character (cast `/Game/BlueprintClasses/AI/AI_Characters/EnemyChaserStatue/BP_AI_enemyChaserStatueCharacter` Agent))
  (bind _neededvelocity (`self.Jump Velocity` Destination (`self.K2_GetActorLocation` Agent) (`self.TotalJumpDuration`)))
  (`Character.LaunchCharacter` _asbp_ai_enemy_chaser_statue_character _neededvelocity true true))

(fn `Jump Velocity`
  (params (EndLocation :type "Vector Structure") (StartLocation :type "Vector Structure") (Duration :type "Float (double-precision)"))
  (returns (NeededVelocity :type "Vector Structure"))
  (locals (LDuration :type "Float (double-precision)"))
  (set `local.LDuration` Duration)
  (return (`KismetMathLibrary.MakeVector` (/ (- (.x EndLocation) (.x StartLocation)) (`local.LDuration`)) (/ (- (.y EndLocation) (.y StartLocation)) (`local.LDuration`)) (/ (- (.z EndLocation) (+ (.z StartLocation) (* (`KismetMathLibrary.Square` (`local.LDuration`)) -0.5 982.0))) (`local.LDuration`)))))

(fn `UserConstructionScript`)