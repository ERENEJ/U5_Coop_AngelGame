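; Enemy chaser statue AI character whose collision box triggers the lose screen when it overlaps a player.
; Standalone play shows it immediately; multiplayer shows it to all players only if another player has zero health.
; Unused eye-contact logic, noted as moved to C++, combines visibility traces with a view-angle check to set the blackboard's IsObserved key on the server.
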(event `Set Inıtıal ValuesFromServer`
  ;[1 0 0] NOT in USE!! Moved  all this logic to c++ they are here for doumantation reasons
  ;;[1 1 1] Setting base values on server with out replcation each client  starts to have their own helper angel
  ;;;[1 0 0.4674] Does not get all player refs only gets the server
  (bind _outactors (`GameplayStatics.GetAllActorsOfClass` "/Game/BlueprintClasses/CharacterBase/BP_CharacterBase.BP_CharacterBase_C"))
  (set `self.BP Character Base REFs(not used)` _outactors))

(event `SR_Follow Player and turn face to target`
  ;[1 0 0] NOT in USE!! Moved  all this logic to c++ they are here for doumantation reasons
  ;;[1 1 1] follow player (will be located in back of the player with is seen check)
  (if (`|EnumEquality` (`self.GetLocalRole`) "ROLE_Authority")
    (bind _eyecontact (`self.IsThereA EyeContactWithAnyPlayer`))
    (`BlackboardComponent.SetValueAsBool` (`AIBlueprintHelperLibrary.GetBlackboard` null) "IsObserved" (not _eyecontact))))

(event `self.ReceiveBeginPlay`
  ;[1 0 0] NOT in USE!! Moved  all this logic to c++ they are here for doumantation reasons
)

(event `self.ReceiveTick`
  (params (DeltaSeconds :type "Float (single-precision)"))
  ;[1 0 0] NOT in USE!! Moved  all this logic to c++ they are here for doumantation reasons
)

(event `self.CollisionBox.OnComponentBeginOverlap`
  (params (OverlappedComponent :type "PrimitiveComponent Object Reference") (OtherActor :type "Actor Object Reference") (OtherComp :type "PrimitiveComponent Object Reference") (OtherBodyIndex :type Integer) (bFromSweep :type Boolean) (SweepResult :type "HitResult Structure (by ref)"))
  ;[0 1 0.1877] Used For Dead/Lose Screen Logic
  (bind _asbp_character_base (cast `/Game/BlueprintClasses/CharacterBase/BP_CharacterBase` OtherActor))
  (`/Engine/EditorBlueprintResources/StandardMacros.IsValid` _asbp_character_base
    (:`Is Valid`
      (if (`KismetSystemLibrary.IsStandalone`)
        (`/Game/BlueprintClasses/CharacterBase/BP_CharacterBase.ROC_ AddLoseWidget` _asbp_character_base)
        (else
          (bind _outactors (`GameplayStatics.GetAllActorsOfClass` "/Game/BlueprintClasses/CharacterBase/BP_CharacterBase.BP_CharacterBase_C"))
          (for _array_element _outactors
            (if (and (!= _array_element _asbp_character_base) (== (`CharacterBase.GetHealthPercentage` _array_element) 0.0))
              (for _array_element_2 _outactors
                (`/Engine/EditorBlueprintResources/StandardMacros.IsValid` _array_element_2
                  (:`Is Valid`
                    (`/Game/BlueprintClasses/CharacterBase/BP_CharacterBase.ROC_ AddLoseWidget` _array_element_2)))))))))))

(fn `IsThereA EyeContactWithAnyPlayer`
  (returns (EyeContact :type Boolean))
  (for _array_element (`self.BP Character Base REFs(not used)`)
    (bind (_outhit _returnvalue) (`KismetSystemLibrary.LineTraceSingle` :`Start` (`self.K2_GetActorLocation` self) :`End` (`self.GetActorEyesViewPoint` _array_element) :`TraceChannel` "TraceTypeQuery1" :`DrawDebugType` "ForDuration" :`DrawTime` 3.0))
    (if (and (> (`KismetMathLibrary.DegAcos` (`KismetMathLibrary.VSize` (- (`KismetMathLibrary.Normal` (- (`self.K2_GetActorLocation`) (`self.K2_GetActorLocation` _array_element)) 0.0) (`SceneComponent.GetForwardVector` (`Actor.RootComponent` _array_element))))) 30.0) (not _returnvalue))
      (`KismetSystemLibrary.PrintString` "EYE CONTACT" true true (struct :`R` 1.0 :`B` 0.75 :`A` 1.0) 5.0)
      (`KismetSystemLibrary.PrintString` "early return")
      (return true)))
  ;[1 1 1] Comment
  (`KismetSystemLibrary.PrintString` "array loop completed")
  (`KismetSystemLibrary.PrintString` "NO EYE CONTACT" true true (struct :`R` 1.0 :`B` 0.032916 :`A` 1.0) 5.0)
  (return false))

(fn `UserConstructionScript`)