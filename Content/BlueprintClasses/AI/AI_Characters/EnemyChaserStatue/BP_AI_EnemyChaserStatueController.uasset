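; AI controller for the chaser statue enemy, which starts its behavior tree on BeginPlay.
; When AI perception successfully senses a player character, it passes it to the controlled statue's chaser target queue.
; Sensed placeable items reach only an empty cast, reserved for destroying spawner totems later.
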(event `self.ReceiveBeginPlay`
  (`parent.ReceiveBeginPlay`)
  (`self.RunBehaviorTree` "/Game/BlueprintClasses/AI/AI_Characters/EnemyChaserStatue/BT_EnemyChaserStatue.BT_EnemyChaserStatue"))

(event `self.AIPerception.OnTargetPerceptionUpdated`
  (params (Actor :type "Actor Object Reference") (Stimulus :type "AIStimulus Structure"))
  (if Stimulus_bSuccessfullySensed
    (bind _asbp_character_base (cast `/Game/BlueprintClasses/CharacterBase/BP_CharacterBase` Actor)
      (:`then`
        (bind _asbp_ai_enemy_chaser_statue_character (cast `/Game/BlueprintClasses/AI/AI_Characters/EnemyChaserStatue/BP_AI_enemyChaserStatueCharacter` (`self.K2_GetPawn`)))
        (`AI_EnemyChaserStatueBase.AddTargetPlayerToChaserQueue` _asbp_ai_enemy_chaser_statue_character _asbp_character_base))
      (:`CastFailed`
        ;[1 1 1] will be used to destroy spawner  totems that can can be seen in the feature
        (cast `/Game/BlueprintClasses/PlaceableItems/BP_PlaceableItem` Actor)))))

(fn `UserConstructionScript`
  (`parent.UserConstructionScript`))