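; Behavior tree task that moves an AI pawn toward its TargetActor, failing if that blackboard actor is invalid.
; It projects a point a fixed distance from SelfActor along the direction to the target, with height zeroed.
; AIMoveTo heads to a random reachable point around that projection, rather than computing a closest one.
; The move's outcome finishes the task, but an invalid AI controller leaves it unfinished.
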(event `self.ReceiveExecute`
  (params (OwnerActor :type "Actor Object Reference"))
  (bind _returnvalue (`AIBlueprintHelperLibrary.GetAIController` OwnerActor))
  (bind _returnvalue_2 (`BTFunctionLibrary.GetBlackboardValueAsActor` (make `BlackboardKeySelector` _ "SelfActor")))
  (bind _returnvalue_3 (`BTFunctionLibrary.GetBlackboardValueAsActor` (make `BlackboardKeySelector` _ "TargetActor")))
  (bind (_returnvalue_x _returnvalue_y) (`KismetMathLibrary.BreakVector` (`Actor.K2_GetActorLocation` _returnvalue_2)))
  (bind (_returnvalue_x_2 _returnvalue_y_2) (`KismetMathLibrary.BreakVector` (`KismetMathLibrary.GetDirectionUnitVector` (`Actor.K2_GetActorLocation` _returnvalue_2) (`Actor.K2_GetActorLocation` _returnvalue_3))))
  (`/Engine/EditorBlueprintResources/StandardMacros.IsValid` _returnvalue_3
    (:`Is Valid`
      (`/Engine/EditorBlueprintResources/StandardMacros.IsValid` _returnvalue
        (:`Is Valid`
          (`AITask_MoveTo.AIMoveTo` _returnvalue (`NavigationSystemV1.K2_GetRandomReachablePointInRadius` (+ (`KismetMathLibrary.MakeVector` _returnvalue_x _returnvalue_y) (* (`KismetMathLibrary.MakeVector` _returnvalue_x_2 _returnvalue_y_2) 2500.0)) 300.0 null null) null
            (:`OnRequestFailed`
              (`self.FinishExecute` false))
            (:`OnMoveFinished`
              (`self.FinishExecute` true))))))
    (:`Is Not Valid`
      (`self.FinishExecute` false))))