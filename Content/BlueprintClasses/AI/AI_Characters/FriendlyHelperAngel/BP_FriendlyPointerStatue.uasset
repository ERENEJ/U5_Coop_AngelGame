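; BP_FriendlyPointerStatue is a helper angel statue meant to trail players and face the target item nearest their last known location.
; A looping timer writes a player's location to the Blackboard after significant movement.
; An eye-contact check using line traces and view direction sets IsObserved and gates rotation toward the target.
; BeginPlay and Tick are empty, with the setup and update calls left disconnected.
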(event `Set Inıtıal ValuesFromServer`
  ;[1 1 1] Setting base values on server with out replcation each client  starts to have their own helper angel
  ;;[1 0 0.4674] Does not get all player refs only gets the server
  (bind _outactors (`GameplayStatics.GetAllActorsOfClass` "/Game/BlueprintClasses/CharacterBase/BP_CharacterBase.BP_CharacterBase_C"))
  (bind _output_get (set `self.BP_CharacterBase_REFs` _outactors))
  (bind _outitem (`KismetArrayLibrary.Array_Random` _output_get))
  (`/Engine/EditorBlueprintResources/StandardMacros.IsValid` _outitem
    (:`Is Valid`
      (set `self.Previous Player Location` (`self.K2_GetActorLocation` _outitem)))))

(event `self.ReceiveBeginPlay`
  ;[1 1 1] Complete Target Totem Selection logic
)

(event `UpdateFriendlyAngel`
  ;[1 1 1] Complete Target Totem Selection logic
  ;;[1 1 1] to compare distance
  ;; instead of writing some large value top of my head I get the one the distance of statues this also work for totem destroy
  (`self.SetBaseDistancetoTargetItem`)
  ;;[1 1 1] instead of getting all the actors set a logic where a target item is removed from array
  (bind _outactors (`GameplayStatics.GetAllActorsOfClass` "/Game/BlueprintClasses/PickableItems/TargetItem/BP_TargetItem.BP_TargetItem_C"))
  (for _array_element _outactors
    (bind _returnvalue (`KismetMathLibrary.Vector_DistanceSquared` (`self.K2_GetActorLocation` _array_element) (`self.Previous Player Location`)))
    (if (<= _returnvalue (`self.tempDistanceHolder`))
      (set `self.tempDistanceHolder` _returnvalue)
      (set `self.CurrentTargetItem_0` _array_element)))
  (`self.SR_Follow Player and turn face to target`))

(event `SR_Get Old Player Location`
  ;[0.9835 0.01151 1] new place
  ;;[1 1 1] Comment
  (`KismetSystemLibrary.K2_SetTimerDelegate` (delegate `CustomEvent_0`) 3.0 true))

(event `CustomEvent_0`
  ;[0.9835 0.01151 1] new place
  ;;[1 1 1] finding first char for now
  (for _array_element (`self.BP_CharacterBase_REFs`)
    (`/Engine/EditorBlueprintResources/StandardMacros.IsValid` _array_element
      (:`Is Valid`
        (break))))
  (`/Engine/EditorBlueprintResources/StandardMacros.IsValid` _array_element
    (:`Is Valid`
      (bind _returnvalue (`self.K2_GetActorLocation` _array_element))
      (if (not (== (`self.Previous Player Location`) _returnvalue :`ErrorTolerance` 1500.0))
        (set `self.Previous Player Location` _returnvalue)
        (`BlackboardComponent.SetValueAsVector` (`AIBlueprintHelperLibrary.GetBlackboard` null) "TargetLocation" (`self.Previous Player Location`))))))

(event `SR_Follow Player and turn face to target`
  ;[1 1 1] follow player (will be located in back of the player with is seen check)
  ;;[1 1 1] finding first char for now
  (for _array_element (`self.BP_CharacterBase_REFs`)
    (`/Engine/EditorBlueprintResources/StandardMacros.IsValid` _array_element
      (:`Is Valid`
        (break))))
  (`/Engine/EditorBlueprintResources/StandardMacros.IsValid` _array_element
    (:`Is Valid`
      (bind _eyecontact (`self.IsThereA EyeContactWithAnyPlayer`))
      (bind _returnvalue (not _eyecontact))
      (`BlackboardComponent.SetValueAsBool` (`AIBlueprintHelperLibrary.GetBlackboard` null) "IsObserved" _returnvalue)
      (if _returnvalue
        (`self.FaceTowardsTargetItem`)))))

(event `FaceTowardsTargetItem`
  ;[1 1 1] FaceForward to target totem
  (`/Engine/EditorBlueprintResources/StandardMacros.IsValid` (`self.CurrentTargetItem_0`)
    (:`Is Valid`
      (`self.K2_SetActorRotation` (`KismetMathLibrary.FindLookAtRotation` (`self.K2_GetActorLocation` self) (`self.K2_GetActorLocation` (`self.CurrentTargetItem_0`)))))))

(event `self.ReceiveTick`
  (params (DeltaSeconds :type "Float (single-precision)")))

(fn `IsThereA EyeContactWithAnyPlayer`
  (returns (EyeContact :type Boolean))
  (for _array_element (`self.BP_CharacterBase_REFs`)
    (bind (_outhit _returnvalue) (`KismetSystemLibrary.LineTraceSingle` :`Start` (`self.K2_GetActorLocation` self) :`End` (`self.GetActorEyesViewPoint` _array_element) :`TraceChannel` "TraceTypeQuery1" :`DrawTime` 3.0))
    (if (and (> (`KismetMathLibrary.DegAcos` (`KismetMathLibrary.VSize` (- (`KismetMathLibrary.Normal` (- (`self.K2_GetActorLocation`) (`self.K2_GetActorLocation` _array_element)) 0.0) (`SceneComponent.GetForwardVector` (`Actor.RootComponent` _array_element))))) 30.0) (not _returnvalue))
      (return true)))
  (return false))

(fn `SetBaseDistancetoTargetItem`
  (bind _returnvalue (`GameplayStatics.GetActorOfClass` "/Game/BlueprintClasses/PickableItems/TargetItem/BP_TargetItem.BP_TargetItem_C"))
  (set `self.tempDistanceHolder` (`self.GetSquaredDistanceTo` _returnvalue self)))

(fn `UserConstructionScript`)