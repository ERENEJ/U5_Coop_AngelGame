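; BP_TargetItem is a collectible objective item that counts toward a win condition when interacted with.
; On interaction it increments the found-item total on every BP_CharacterBase in the world, so progress is shared rather than credited to the interactor.
; Any character whose total reaches five gets ROCAddWinWidget called to add the win widget, then the item destroys itself.
; It reports itself as not possessable.
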(event `InteractionInterface.InteractWithActor`
  (params (InteractionCaller :type "Pawn Object Reference"))
  (bind _outactors (`GameplayStatics.GetAllActorsOfClass` "/Game/BlueprintClasses/CharacterBase/BP_CharacterBase.BP_CharacterBase_C"))
  (for _array_element _outactors
    (`/Engine/EditorBlueprintResources/StandardMacros.IsValid` _array_element
      (:`Is Valid`
        (bind _result (`/Engine/EditorBlueprintResources/StandardMacros.IncrementInt` (`CharacterBase.TotalFoundTargetItemAmount` _array_element))
          (:`  `
            (if (== _result 5)
              (`/Game/BlueprintClasses/CharacterBase/BP_CharacterBase.ROC_Add Win Widget` _array_element)))))))
  (`self.K2_DestroyActor`))

(fn `IsPossessable`
  (returns (ReturnValue :type Boolean))
  (return false))

(fn `UserConstructionScript`)