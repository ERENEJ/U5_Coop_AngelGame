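; BP_CharacterBase is a first-person character Blueprint that handles the end-of-match win and lose screens.
; The ROC_AddWinWidget and ROC_AddLoseWidget events show BP_YouWin or BP_YouLose through BP_FPS_PlayerController, remove it after a short delay, then call ReturnToMainMenuHost where a GameMode is valid.
; The F key runs a debug camera line trace that prints the hit component's name.
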(event `Key|F`
  (params (Key :type "Key Structure"))
  (bind _firstpersoncameracomponent (`self.FirstPersonCameraComponent`))
  (bind (_returnvalue_x _returnvalue_y _returnvalue_z) (`KismetMathLibrary.BreakVector` (`SceneComponent.GetForwardVector` _firstpersoncameracomponent)))
  (bind _returnvalue (`SceneComponent.K2_GetComponentLocation` _firstpersoncameracomponent))
  (:`Pressed`
    ;[1 0.04114 0.03119] This only for debug purpose no functionalty is hapening here other than single linetrace
    (bind _outhit (`KismetSystemLibrary.LineTraceSingle` :`Start` _returnvalue :`End` (+ _returnvalue (`KismetMathLibrary.MakeVector` (* _returnvalue_x 1000.0) (* _returnvalue_y 1000.0) (* _returnvalue_z 1000.0))) :`TraceChannel` "TraceTypeQuery1" :`DrawDebugType` "ForDuration"))
    (`KismetSystemLibrary.PrintString` (`KismetSystemLibrary.GetDisplayName` (`.HitComponent` (`GameplayStatics.BreakHitResult` _outhit))) true true (struct :`G` 0.66 :`B` 1.0 :`A` 1.0) 15.0)))

(event `ROC_Add Win Widget`
  (bind _returnvalue (`GameplayStatics.GetGameMode`))
  (bind _asbp_fps_player_controller (cast `/Game/BlueprintClasses/BP_FPS_PlayerController` (`self.GetController`)))
  (bind _returnvalue_2 (`|CreateWidget` "/Game/BlueprintClasses/UI/BP_YouWin.BP_YouWin_C" _asbp_fps_player_controller))
  (`UserWidget.AddToViewport` _returnvalue_2 0)
  (`KismetSystemLibrary.Delay` 3.0)
  (`Widget.RemoveFromParent` _returnvalue_2)
  (`/Engine/EditorBlueprintResources/StandardMacros.IsValid` _returnvalue
    (:`Is Valid`
      (`GameModeBase.ReturnToMainMenuHost` _returnvalue))))

(event `ROC_ AddLoseWidget`
  (bind _returnvalue (`GameplayStatics.GetGameMode`))
  (bind _asbp_fps_player_controller (cast `/Game/BlueprintClasses/BP_FPS_PlayerController` (`self.GetController`)))
  (bind _returnvalue_2 (`|CreateWidget` "/Game/BlueprintClasses/UI/BP_YouLose.BP_YouLose_C" _asbp_fps_player_controller))
  (`UserWidget.AddToViewport` _returnvalue_2 0)
  (`KismetSystemLibrary.Delay` 3.0)
  (`Widget.RemoveFromParent` _returnvalue_2)
  (`/Engine/EditorBlueprintResources/StandardMacros.IsValid` _returnvalue
    (:`Is Valid`
      (`GameModeBase.ReturnToMainMenuHost` _returnvalue))))

(fn `UserConstructionScript`)