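; Usable voodoo item that shows a ghost preview of where the voodoo doll will be placed.
; From BeginPlay, a self-repeating delayed loop line-traces forward from the Arrow, spawning or moving a collisionless preview actor at the hit and updating SpawnAllowed.
; The preview is removed when the trace misses, the item is placed or the item is destroyed.
; Spawning the real placeable is marked as moved to C++, leaving its Blueprint event uncalled here.
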(event `sr_spawndool`
  ;[0 0.9085 1] Moved to c++
  (bind _returnvalue (`|SpawnActorFromClass` "/Game/BlueprintClasses/PlaceableItems/BP_PlaceableItem.BP_PlaceableItem_C" (`KismetMathLibrary.MakeTransform` (`self.VoodooSpawnLocation`) (`self.VoodooSpawnRotation`)) "Undefined" "OverrideRootScale" (`self.GetOwner`) null))
  (`self.SetActorScale3D` _returnvalue (3.0 3.0 3.0)))

(event `self.ReceiveBeginPlay`
  ;[1 1 1] for creating the ghost item
  (`/Engine/EditorBlueprintResources/StandardMacros.DoOnce` false
    (:`Completed`
      (`self.ItemGhostOverSpawn`))))

(event `ItemGhostOverSpawn`
  (bind (_returnvalue_roll _returnvalue_pitch _returnvalue_yaw) (`KismetMathLibrary.BreakRotator` (`self.K2_GetActorRotation`)))
  (bind _arrow (`self.Arrow`))
  (bind _returnvalue (`SceneComponent.K2_GetComponentLocation` _arrow))
  ;[1 1 1] for creating the ghost item
  (if (`self.bIsPlaced`)
    (`/Engine/EditorBlueprintResources/StandardMacros.IsValid` (`self.placed object`)
      (:`Is Valid`
        (`self.K2_DestroyActor` (`self.placed object`))))
    (else
      (`KismetSystemLibrary.Delay` 0.1)
      (bind (_outhit _returnvalue_2) (`KismetSystemLibrary.LineTraceSingle` _returnvalue (+ _returnvalue (* (`SceneComponent.GetForwardVector` _arrow) 300.0)) "TraceTypeQuery1"))
      (if _returnvalue_2
        (set `self.VoodooSpawnLocation` (`.Location` (`GameplayStatics.BreakHitResult` _outhit)))
        ;;[1 1 1] to face where we are looking at
        (set `self.VoodooSpawnRotation` (`KismetMathLibrary.MakeRotator` 0.0 0.0 _returnvalue_yaw))
        ;;[1 0 0] UNPLUG here for removing ghot item/placement indicator
        (`/Engine/EditorBlueprintResources/StandardMacros.IsValid` (`self.placed object`)
          (:`Is Valid`
            ;;[1 1 1] we are spawning translucent object once and keep changing location of it
            (`self.K2_SetActorLocation` (`self.placed object`) (`self.VoodooSpawnLocation`) false false)
            (`self.ItemGhostOverSpawn`))
          (:`Is Not Valid`
            (bind _returnvalue_3 (`|SpawnActorFromClass` "/Game/BlueprintClasses/PlaceableItems/BP_PreviewPlaceableItem.BP_PreviewPlaceableItem_C" (`KismetMathLibrary.MakeTransform` (`self.VoodooSpawnLocation`) (`self.VoodooSpawnRotation`)) "Undefined" "OverrideRootScale" self null))
            (bind _output_get (set `self.placed object` _returnvalue_3))
            (`/Engine/EditorBlueprintResources/StandardMacros.IsValid` _output_get
              (:`Is Valid`
                (`self.SetActorEnableCollision` _output_get false)
                (set `self.bSpawnAllowed` true)
                (`self.ItemGhostOverSpawn`)))))
        (else
          (`/Engine/EditorBlueprintResources/StandardMacros.IsValid` (`self.placed object`)
            (:`Is Valid`
              (`self.K2_DestroyActor` (`self.placed object`))
              (set `self.bSpawnAllowed` false)
              (`self.ItemGhostOverSpawn`))
            (:`Is Not Valid`
              (set `self.bSpawnAllowed` false)
              (`self.ItemGhostOverSpawn`))))))))

(event `self.ReceiveEndPlay`
  (params (EndPlayReason :type "EEndPlayReason Enum" :default "Destroyed"))
  (bind _placed_object (`self.placed object`))
  (switch `EEndPlayReason` EndPlayReason
    (:`Destroyed`
      (`/Engine/EditorBlueprintResources/StandardMacros.IsValid` _placed_object
        (:`Is Valid`
          (`self.K2_DestroyActor` _placed_object))))))

(fn `UserConstructionScript`)