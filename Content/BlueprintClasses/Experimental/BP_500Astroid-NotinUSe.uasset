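; Experimental asteroid field, named as not in use, that scatters about 5,000 randomly placed, rotated and scaled asteroids as hierarchical instanced meshes.
; The construction script builds the instances in local space.
; Despite their names, the Start/Stop rotation events play or stop a timeline that offsets the root along local X and Y.
; Box overlaps are empty; the spaceship-triggered start/stop logic and older rotation method are disconnected.
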(event `StartAstroidRotation`
  (bind (_direction _newtrack_1) (`Timeline|Timeline_0` :!label _label)
    (:`Update`
      (bind _returnvalue (* _newtrack_1 100.0))
      (`SceneComponent.K2_AddLocalOffset` (`self.DefaultSceneRoot`) (`KismetMathLibrary.MakeVector` _returnvalue _returnvalue) false false))))

(event `StopAstroidRotation`
  (goto _label :!via `Stop`))

(event `self.Box.OnComponentBeginOverlap`
  (params (OverlappedComponent :type "PrimitiveComponent Object Reference") (OtherActor :type "Actor Object Reference") (OtherComp :type "PrimitiveComponent Object Reference") (OtherBodyIndex :type Integer) (bFromSweep :type Boolean) (SweepResult :type "HitResult Structure (by ref)")))

(event `self.Box.OnComponentEndOverlap`
  (params (OverlappedComponent :type "PrimitiveComponent Object Reference") (OtherActor :type "Actor Object Reference") (OtherComp :type "PrimitiveComponent Object Reference") (OtherBodyIndex :type Integer)))

(fn `UserConstructionScript`
  (bind _returnvalue (`KismetMathLibrary.RandomFloatInRange` 0.0 360.0))
  (for _ (range 5001)
    (`InstancedStaticMeshComponent.AddInstance` (`self.HierarchicalInstancedStaticMesh`) (`KismetMathLibrary.MakeTransform` (`KismetMathLibrary.MakeVector` (* 10.0 (`KismetMathLibrary.RandomFloatInRange` 200.0 6000.0)) (* 10.0 (`KismetMathLibrary.RandomFloatInRange` 200.0 5000.0)) (`KismetMathLibrary.RandomFloatInRange` 0.0 10000.0)) (`KismetMathLibrary.MakeRotator` _returnvalue _returnvalue) (`KismetMathLibrary.MakeVector` (`KismetMathLibrary.RandomFloatInRange` 3.0 4.0) (`KismetMathLibrary.RandomFloatInRange` 4.0 5.0) (`KismetMathLibrary.RandomFloatInRange` 3.0 4.0))) false)))