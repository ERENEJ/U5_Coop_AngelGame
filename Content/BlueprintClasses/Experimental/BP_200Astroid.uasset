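; Experimental asteroid field actor that scatters randomly placed, rotated and scaled instanced meshes in its construction script, with collision initially off.
; A timeline started at BeginPlay drifts the root along local X and Y, despite the "rotation" event names.
; Box overlaps with specific ship and projectile classes adjust a counter, enabling mesh collision on entry and disabling it at zero.
; The begin and end class checks differ, so the count can become unbalanced.
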(event `self.ReceiveBeginPlay`
  (`self.StartAstroidRotation`))

(event `StartAstroidRotation`
  (bind (_direction _newtrack_1) (`Timeline|Timeline_0` :!label _label)
    (:`Update`
      (bind _returnvalue (* _newtrack_1 200.0))
      (`SceneComponent.K2_AddLocalOffset` (`self.DefaultSceneRoot`) (`KismetMathLibrary.MakeVector` _returnvalue _returnvalue) false false))))

(event `StopAstroidRotation`
  (goto _label :!via `Stop`))

(event `self.Box.OnComponentBeginOverlap`
  (params (OverlappedComponent :type "PrimitiveComponent Object Reference") (OtherActor :type "Actor Object Reference") (OtherComp :type "PrimitiveComponent Object Reference") (OtherBodyIndex :type Integer) (bFromSweep :type Boolean) (SweepResult :type "HitResult Structure (by ref)"))
  (bind _returnvalue (`GameplayStatics.GetObjectClass` OtherActor))
  (if (or (== _returnvalue "/Game/BlueprintClasses/Vehicles/BP_MasterSpaceShip.BP_MasterSpaceShip_C") (== _returnvalue "/Game/BlueprintClasses/Projectile/BP_AstroidTunnelProjectile.BP_AstroidTunnelProjectile_C") (== _returnvalue "/Game/BlueprintClasses/Vehicles/BP_SpaceShip_Child.BP_SpaceShip_Child_C"))
    (`PrimitiveComponent.SetCollisionEnabled` (`self.HierarchicalInstancedStaticMesh`) "QueryAndPhysics")
    (`/Engine/EditorBlueprintResources/StandardMacros.IncrementInt` (`self.Objectnumber`))))

(event `self.Box.OnComponentEndOverlap`
  (params (OverlappedComponent :type "PrimitiveComponent Object Reference") (OtherActor :type "Actor Object Reference") (OtherComp :type "PrimitiveComponent Object Reference") (OtherBodyIndex :type Integer))
  (bind _returnvalue (`GameplayStatics.GetObjectClass` OtherActor))
  (if (or (== _returnvalue "/Script/ProjectFPS.SpaceShipBase") (== _returnvalue "/Game/BlueprintClasses/Projectile/BP_AstroidTunnelProjectile.BP_AstroidTunnelProjectile_C") (== _returnvalue "/Game/BlueprintClasses/Vehicles/BP_MasterSpaceShip.BP_MasterSpaceShip_C"))
    (bind _result (`/Engine/EditorBlueprintResources/StandardMacros.DecrementInt` (`self.Objectnumber`))
      (:`  `
        (if (== _result 0)
          (`PrimitiveComponent.SetCollisionEnabled` (`self.HierarchicalInstancedStaticMesh`) "NoCollision"))))))

(fn `UserConstructionScript`
  (bind _returnvalue (`KismetMathLibrary.RandomFloatInRange` 0.0 360.0))
  (for _ (range 201)
    (`InstancedStaticMeshComponent.AddInstance` (`self.HierarchicalInstancedStaticMesh`) (`KismetMathLibrary.MakeTransform` (`KismetMathLibrary.MakeVector` (* 13.0 (`KismetMathLibrary.RandomFloatInRange` 200.0 2500.0)) (* 13.0 (`KismetMathLibrary.RandomFloatInRange` 200.0 2500.0)) (`KismetMathLibrary.RandomFloatInRange` 0.0 35000.0)) (`KismetMathLibrary.MakeRotator` _returnvalue _returnvalue) (`KismetMathLibrary.MakeVector` (`KismetMathLibrary.RandomFloatInRange` 10.0 15.0) (`KismetMathLibrary.RandomFloatInRange` 10.0 15.0) (`KismetMathLibrary.RandomFloatInRange` 10.0 15.0))) false)
    (`PrimitiveComponent.SetCollisionEnabled` (`self.HierarchicalInstancedStaticMesh`) "NoCollision")))