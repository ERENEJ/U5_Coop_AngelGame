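; BP_MapItemCreator randomly populates the map with craft materials, observer statues and target items at BeginPlay, using painted foliage as spawn points.
; SR_SpawnItem walks every instance in the first InstancedFoliageActor's foliage components and makes weighted random rolls.
; A small share yields either alternating craft materials (via FlipFlop) or AI-spawned BP_ObserverStatue pawns.
; The remainder rarely yield a half-scale BP_TargetItem at fixed height, capped by TargetItemCount.
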(event `self.ReceiveBeginPlay`
  (`self.SR_Spawn Item`))

(event `SR_Spawn Item`
  (bind _returnvalue (`GameplayStatics.GetActorOfClass` "/Script/Foliage.InstancedFoliageActor"))
  (`/Engine/EditorBlueprintResources/StandardMacros.IsValid` _returnvalue
    (:`Is Valid`
      (for _array_element (`self.K2_GetComponentsByClass` _returnvalue "/Script/Foliage.FoliageInstancedStaticMeshComponent")
        (for _index (range (`InstancedStaticMeshComponent.GetInstanceCount` _array_element))
          (if (`KismetMathLibrary.RandomBoolWithWeight` 0.02)
            (if (`KismetMathLibrary.RandomBool`)
              (`/Engine/EditorBlueprintResources/StandardMacros.FlipFlop`
                (:`A`
                  (bind _location (.location (`InstancedStaticMeshComponent.GetInstanceTransform` _array_element _index false)))
                  (`|SpawnActorFromClass` "/Game/BlueprintClasses/PickableItems/BP_CraftMaterial1.BP_CraftMaterial1_C" (`KismetMathLibrary.MakeTransform` _location) "AlwaysSpawn" "OverrideRootScale" null null))
                (:`B`
                  (`|SpawnActorFromClass` "/Game/BlueprintClasses/PickableItems/BP_CraftMaterial2.BP_CraftMaterial2_C" (`KismetMathLibrary.MakeTransform` _location) "AlwaysSpawn" "OverrideRootScale" null null)))
              (else
                (`AIBlueprintHelperLibrary.SpawnAIFromClass` "/Game/BlueprintClasses/AI/AI_Characters/PlacedObserverStatue/BP_ObserverStatue.BP_ObserverStatue_C" null (+ _location (50.0 50.0 100.0)) (.rotation (`InstancedStaticMeshComponent.GetInstanceTransform` _array_element _index false)) false null)))
            (elif (and (`KismetMathLibrary.RandomBoolWithWeight` 0.002) (< (`self.TargetItemCount`) 6))
              (bind (_x _y) (`KismetMathLibrary.BreakVector3f` _location))
              (`|SpawnActorFromClass` "/Game/BlueprintClasses/PickableItems/TargetItem/BP_TargetItem.BP_TargetItem_C" (`KismetMathLibrary.MakeTransform` (`KismetMathLibrary.MakeVector` _x _y 400.0) (struct) (0.5 0.5 0.5)) "AlwaysSpawn" "OverrideRootScale" null null)
              (`/Engine/EditorBlueprintResources/StandardMacros.IncrementInt` (`self.TargetItemCount`)))))))))

(fn `UserConstructionScript`)