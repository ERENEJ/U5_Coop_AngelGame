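; Child spaceship Blueprint that hands player control to a companion ship unit when its energy runs out.
; On BeginPlay it calls SR_Spawn to spawn that unit at the plane mesh's location, unattached, plus two attached doors.
; Tick watches EnergyValue; at zero or below, the FPS player controller possesses the unit.
; SR_AddComponents, meant for the server, then gives it replicated rotation and movement components.
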(event `self.ReceiveBeginPlay`
  (`parent.ReceiveBeginPlay`)
  (`KismetSystemLibrary.PrintString` "begin play" true true (struct :`G` 0.66 :`B` 1.0 :`A` 1.0) 200.0)
  (`self.SR_Spawn`))

(event `SR_Spawn`
  (bind _returnvalue (`|SpawnActorFromClass` "/Game/BlueprintClasses/ShipUnits/BP_SpaceShipUnit_Child.BP_SpaceShipUnit_Child_C" (`KismetMathLibrary.Conv_VectorToTransform` (`SceneComponent.K2_GetComponentLocation` (`self.PlaneMesh`))) "AlwaysSpawn" "OverrideRootScale" self null))
  (bind _output_get (set `self.ShipUnit` _returnvalue))
  ;[1 1 1] outer door
  (bind _returnvalue_2 (`|SpawnActorFromClass` "/Game/BlueprintClasses/Vehicles/BP_ShipDoor.BP_ShipDoor_C" (`KismetMathLibrary.Conv_VectorToTransform` (`SceneComponent.K2_GetComponentLocation` (`self.doorLocation`))) "AlwaysSpawn" "OverrideRootScale" self null))
  (`self.K2_AttachToComponent` _returnvalue_2 (`self.doorLocation`) "None" "SnapToTarget" "KeepRelative" "KeepRelative" true)
  ;[1 1 1] inner door
  (bind _returnvalue_3 (`|SpawnActorFromClass` "/Game/BlueprintClasses/Vehicles/BP_ShipDoor.BP_ShipDoor_C" (`KismetMathLibrary.Conv_VectorToTransform` (`SceneComponent.K2_GetComponentLocation` (`self.doorLocation`))) "AlwaysSpawn" "OverrideRootScale" self null))
  (`self.K2_AttachToComponent` _returnvalue_3 (`self.doorLocation1Part2`) "None" "SnapToTarget" "KeepRelative" "KeepRelative" true))

(event `self.ReceiveTick`
  (params (DeltaSeconds :type "Float (single-precision)"))
  (`parent.ReceiveTick` DeltaSeconds)
  ;[1 1 1] Need to handle death events on take damage
  (if (<= (`self.EnergyValue`) 0.0)
    (bind _asbp_fps_player_controller (cast `/Game/BlueprintClasses/BP_FPS_PlayerController` (`Pawn.GetController`)))
    (`Controller.Possess` _asbp_fps_player_controller (`self.ShipUnit`))
    (`self.SR_AddComponents`)))

(event `SR_AddComponents`
  (bind _shipunit (`self.ShipUnit`))
  ;[1 1 1] Need to call this part on server for non replicated client errors(to reduce runtime errors)
  (bind _returnvalue (`AddComponent|NODE_AddRotationComponent-1` :`self` _shipunit))
  (`ActorComponent.SetIsReplicated` _returnvalue true)
  (`SpaceShipUnitBase.SetRotationComponent` _shipunit _returnvalue)
  (bind _returnvalue_2 (`AddComponent|NODE_AddShipMovementComponent-0` :`self` _shipunit))
  (`ActorComponent.SetIsReplicated` _returnvalue_2 true)
  (`SpaceShipUnitBase.SetShipMovementComponent` _shipunit _returnvalue_2))

(fn `UserConstructionScript`
  (`parent.UserConstructionScript`))