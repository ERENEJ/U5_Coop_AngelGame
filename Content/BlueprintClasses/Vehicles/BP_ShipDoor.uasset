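; BP_ShipDoor is an interactable, non-possessable ship door that slides along local Z and returns automatically.
; InteractwithActor plays a timeline to move the door mesh, waits, then plays a second timeline with negated output to reverse it.
; Timeline values are added as per-update local offsets rather than absolute positions, so travel depends on update count.
; Timelines are rewound with SetNewTime; nodes toggling collision and visibility are unconnected.
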(event `InteractionInterface.InteractWithActor`
  (bind (_direction _newtrack_0) (`Timeline|Timeline_0` :`NewTime` 0.0 :!label _label)
    (:`Update`
      (`SceneComponent.K2_AddLocalOffset` (`self.DoorMesh_0`) (`KismetMathLibrary.MakeVector` 0.0 0.0 _newtrack_0) false false))
    (:`Finished`
      (`KismetSystemLibrary.Delay` 3.0)
      (`|ExecutionSequence`
        (:`then_0`
          (bind (_direction_2 _newtrack_0_2) (`Timeline|Timeline_1` :`NewTime` 0.0 :!label _label_2)
            (:`Update`
              (`|ExecutionSequence`
                (:`then_0`
                  (`SceneComponent.K2_AddLocalOffset` (`self.DoorMesh_0`) (`KismetMathLibrary.MakeVector` 0.0 0.0 (* _newtrack_0_2 -1.0)) false false))))
            (:`Finished`
              (`KismetSystemLibrary.Delay` 0.5)
              (goto _label_2 :!via `SetNewTime`))))
        (:`then_1`
          (goto _label :!via `SetNewTime`))))))

(fn `IsPossessable`
  (returns (ReturnValue :type Boolean))
  (return false))

(fn `UserConstructionScript`)