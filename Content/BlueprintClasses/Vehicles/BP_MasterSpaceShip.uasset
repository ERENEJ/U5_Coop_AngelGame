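; BP_MasterSpaceShip is the base spaceship, with an energy pool that powers sprinting and asteroid-tunneling projectiles and takes collision damage.
; Left click fires projectiles from two sockets for an energy cost, on a cooldown.
; Tick drains energy while sprinting, slowly regenerates it otherwise, and jiggles rotation as an asteroid fly-through workaround.
; Box overlaps remove hit HISM instances, shake the camera and cost energy; death and repossession logic is unconnected.
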(event `SR_SpawnProjectile`
  (bind _planemesh (`self.PlaneMesh`))
  (bind _planemesh_2 (`self.PlaneMesh`))
  (if (and (>= (`self.EnergyValue`) 20.0) (`self.bCanFireTunnelingProjectile`))
    (`|SpawnActorFromClass` "/Game/BlueprintClasses/Projectile/BP_AstroidTunnelProjectile.BP_AstroidTunnelProjectile_C" (`KismetMathLibrary.MakeTransform` (`SceneComponent.GetSocketLocation` _planemesh_2 "ProjectileSocket") (`SceneComponent.GetSocketRotation` _planemesh_2 "ProjectileSocket")) "Undefined" "OverrideRootScale" null null)
    (`|SpawnActorFromClass` "/Game/BlueprintClasses/Projectile/BP_AstroidTunnelProjectile.BP_AstroidTunnelProjectile_C" (`KismetMathLibrary.MakeTransform` (`SceneComponent.GetSocketLocation` _planemesh "ProjectileSocket2") (`SceneComponent.GetSocketRotation` _planemesh "ProjectileSocket2")) "Undefined" "OverrideRootScale" null null)
    (set `self.bCanFireTunnelingProjectile` false)
    (set `self.EnergyValue` (- (`self.EnergyValue`) 20.0))
    (`KismetSystemLibrary.Delay` 10.0)
    (set `self.bCanFireTunnelingProjectile` true)))

(event `self.ReceiveTick`
  (params (DeltaSeconds :type "Float (single-precision)"))
  ;[1 1 1] to prevent astroid fly through (quary bug fix)
  (`self.K2_AddActorLocalRotation` (struct :`Roll` 1.0))
  (`self.K2_AddActorLocalRotation` (struct :`Roll` -1.0))
  (if (> (`self.GetInputAxisValue`) 0.01)
    ;[1 1 1] Reduce energy when using shift
    (set `self.EnergyValue` (- (`self.EnergyValue`) DeltaSeconds))
    (else
      ;[1 1 1] Slowly regain energy
      (set `self.EnergyValue` (+ (`self.EnergyValue`) (/ DeltaSeconds 10.0))))))

(event `Key|LeftMouseButton`
  (params (Key :type "Key Structure"))
  (:`Pressed`
    (`self.SR_SpawnProjectile`)))

(event `self.Box.OnComponentBeginOverlap`
  (params (OverlappedComponent :type "PrimitiveComponent Object Reference") (OtherActor :type "Actor Object Reference") (OtherComp :type "PrimitiveComponent Object Reference") (OtherBodyIndex :type Integer) (bFromSweep :type Boolean) (SweepResult :type "HitResult Structure (by ref)"))
  (bind _ashierarchical_instanced_static_mesh_component (cast `HierarchicalInstancedStaticMeshComponent` OtherComp))
  (`InstancedStaticMeshComponent.RemoveInstance` _ashierarchical_instanced_static_mesh_component OtherBodyIndex)
  (`GameplayStatics.PlayWorldCameraShake` "/Game/BlueprintClasses/Experimental/BP_CamShake.BP_CamShake_C" (`self.K2_GetActorLocation`) 0.0 50000.0)
  (bind _output_get (set `self.EnergyValue` (- (`self.EnergyValue`) 20.0)))
  (if (<= _output_get 0.0)
    _))

(fn `GetEnergyPercentage`
  (returns (EnergyValue :type "Float (double-precision)"))
  (return (/ (`self.EnergyValue`) 100.0)))

(fn `UserConstructionScript`)